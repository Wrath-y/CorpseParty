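; Overview display actor that lays out modular zombie skeletal and static meshes in labelled rows, likely as an asset showcase.
; The construction script loops OverviewStructure, spawning a component per mesh at the row offset plus a per-item step, with static meshes continuing after the skeletal ones.
; Each row gets a text label with its name, centered along the row and adjusted by global offset and rotation.
; Event graph is unused.
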(event EventBeginPlay)

(event Collision|EventActorBeginOverlap
  (params (OtherActor :type Actor%20Object%20Reference)))

(event EventTick
  (params (DeltaSeconds :type Float%20%28single-precision%29)))

(fn ConstructionScript
  (bind _globaltextoffset (Variables|Default|GetGlobalTextOffset))
  (for _array_element (Variables|Default|GetOverviewStructure)
    (LocalVariables|SetTempItemOffset (.ItemOffset (Utilities|Struct|BreakStruc_Overview _array_element)))
    (LocalVariables|SetTempRowOffset (+ (.InitialOffset (Utilities|Struct|BreakStruc_Overview _array_element)) (.RowOffset (Utilities|Struct|BreakStruc_Overview _array_element))))
    (Utilities|FlowControl|Sequence
      (:then_0
        (for (_array_element_2 _array_index) (.SkeletalMesh (Utilities|Struct|BreakStruc_Overview _array_element))
          (bind _returnvalue (AddComponent|AddSkeletalMeshComponent false))
          (Components|SkinnedMesh|SetSkinnedAssetandUpdate _returnvalue _array_element_2 true)
          (Components|Animation|SetAnimationMode _returnvalue "AnimationSingleNode" true)
          (Transformation|SetWorldLocation _returnvalue (+ (* (LocalVariables|GetTempItemOffset) _array_index) (Transformation|GetWorldLocation (Variables|Default|GetDefaultSceneRoot)) (LocalVariables|GetTempRowOffset)) false false)))
      (:then_1
        (for (_array_element_3 _array_index_2) (.StaticMesh (Utilities|Struct|BreakStruc_Overview _array_element))
          (bind _returnvalue_2 (AddComponent|AddStaticMeshComponent false))
          (Components|StaticMesh|SetStaticMesh _returnvalue_2 _array_element_3)
          (Transformation|SetWorldLocation _returnvalue_2 (+ (* (LocalVariables|GetTempItemOffset) (+ _array_index_2 (Utilities|Array|Length (.SkeletalMesh (Utilities|Struct|BreakStruc_Overview _array_element))))) (Transformation|GetWorldLocation (Variables|Default|GetDefaultSceneRoot)) (LocalVariables|GetTempRowOffset)) false false)))
      (:then_2
        (bind _returnvalue_3 (AddComponent|AddTextRenderComponent false))
        (Rendering|Components|TextRender|SetWorldSize _returnvalue_3 (Variables|Default|GetTextSize))
        (Rendering|Components|TextRender|SetText _returnvalue_3 (Utilities|Text|ToText(String) (.RowName (Utilities|Struct|BreakStruc_Overview _array_element))))
        (Rendering|Components|TextRender|SetHorizontalAlignment _returnvalue_3 "EHTA_Center")
        (Transformation|SetWorldTransform _returnvalue_3 (Math|Transform|MakeTransform (+ (Math|Vector|MakeVector (.x (+ (/ (* (LocalVariables|GetTempItemOffset) (+ (Utilities|Array|Length (.SkeletalMesh (Utilities|Struct|BreakStruc_Overview _array_element))) (Utilities|Array|Length (.StaticMesh (Utilities|Struct|BreakStruc_Overview _array_element))))) "2.000000,2.000000,1.000000") (Transformation|GetWorldLocation (Variables|Default|GetDefaultSceneRoot)) (+ (.RowOffset (Utilities|Struct|BreakStruc_Overview _array_element)) (.InitialOffset (Utilities|Struct|BreakStruc_Overview _array_element))))) (+ (.y (+ (/ (* (LocalVariables|GetTempItemOffset) (+ (Utilities|Array|Length (.SkeletalMesh (Utilities|Struct|BreakStruc_Overview _array_element))) (Utilities|Array|Length (.StaticMesh (Utilities|Struct|BreakStruc_Overview _array_element))))) "2.000000,2.000000,1.000000") (Transformation|GetWorldLocation (Variables|Default|GetDefaultSceneRoot)) (+ (.RowOffset (Utilities|Struct|BreakStruc_Overview _array_element)) (.InitialOffset (Utilities|Struct|BreakStruc_Overview _array_element))))) (.y _globaltextoffset)) (.z _globaltextoffset)) (* (/ (LocalVariables|GetTempItemOffset) "2.000000,2.000000,2.000000") -1)) (Variables|Default|GetGlobalTextRotation) "1.000000,1.000000,1.000000") false false)))))