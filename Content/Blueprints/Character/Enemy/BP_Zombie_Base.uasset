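; Base zombie enemy character that provides an attack, a patrol route and movement speed control.
; Attack plays the FireWeapon montage on the mesh and calls the OnAttackEnd dispatcher whether it completes or is interrupted.
; GetPatrolRoute returns the stored route, and SetMovementSpeed maps a speed state from idle to sprint onto max walk speed and returns it.
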(event Custom|Attack
  (Animation|Montage|PlayMontage (Variables|Character|GetMesh) "/Game/Blueprints/Character/Player/Animation/FireWeapon.FireWeapon"
    (:OnCompleted
      _)
    (:OnInterrupted
      _))
  (Default|CallOnAttackEnd)
  (Development|PrintString "Attack End"))

(event EventBeginPlay)

(event Collision|EventActorBeginOverlap
  (params (OtherActor :type Actor%20Object%20Reference)))

(event EventTick
  (params (DeltaSeconds :type Float%20%28single-precision%29)))

(fn ConstructionScript
  (|CallParentFunction))

(fn GetPatrolRoute
  (return (Variables|AI|GetPatrolRoute)))

(fn SetMovementSpeed
  (params (Speed :type E_MovementSpeed%20Enum :default "NewEnumerator0"))
  (bind _output_get (Variables|/Script/Engine.CharacterMovementComponent|SetMaxWalkSpeed (Variables|Character|GetCharacterMovement) (Utilities|Select :Index Speed :NewEnumerator0 0.0 :NewEnumerator1 1e+02 :NewEnumerator2 3e+02 :NewEnumerator3 5e+02)))
  (return _output_get))